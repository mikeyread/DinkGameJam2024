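; BP_Master_Enemy is an enemy Blueprint with placeholder wandering that moves it away from its spawner so more can spawn.
; From BeginPlay, TestSpawnerMove sends it to a random reachable point within a radius, then repeats after a short delay on success only.
; Movetofoodbowl is a stub move with no destination set.
; The destroy and OnKilled call nodes are unconnected, so they never run.
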(event Custom|Test%20Spawner%20Move
  ;[1 0.241 0.7891] Simple test movement so enemies move from spawner to allow more to spawn
  (AI|AIMoveTo self (.RandomLocation (AI|Navigation|GetRandomReachablePointinRadius (Transformation|GetActorLocation) 3e+03 0 0)) 0 5.0 false
    (:OnSuccess
      (Utilities|FlowControl|Delay 1.5)
      (CallFunction|TestSpawnerMove))))

(event Custom|Move%20to%20food%20bowl
  (AI|AIMoveTo self "0, 0, 0" 0 5.0 false))

(event EventBeginPlay
  ;[1 0.241 0.7891] Simple test movement so enemies move from spawner to allow more to spawn
  (CallFunction|TestSpawnerMove))

(fn ConstructionScript)