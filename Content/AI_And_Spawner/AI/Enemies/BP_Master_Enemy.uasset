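; Master enemy Blueprint for dog-hunting enemies that chase and "yoink" puppies.
; On BeginPlay it picks a random BPC_BaseDog, registers it in the player's DogsHunted list (checked for duplicates when over five dogs exist) and uses AIMoveTo.
; After arrival and a delay, it unregisters the dog and hunts again.
; Box overlap with the target copies the dog's mesh onto the enemy; attach, kill and wander logic are unwired.
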(event OnComponentBeginOverlap(Box)
  (params (OverlappedComponent :type Primitive%20Component%20Object%20Reference) (OtherActor :type Actor%20Object%20Reference) (OtherComp :type Primitive%20Component%20Object%20Reference) (OtherBodyIndex :type Integer) (bFromSweep :type Boolean) (SweepResult :type Hit%20Result%20Structure%20%28by%20ref%29))
  (bind _dog_granny_is_hunting (Variables|Default|Getdog%20Granny%20is%20hunting))
  (if (== OtherActor _dog_granny_is_hunting)
    (CallFunction|YoinkThatPuppy _dog_granny_is_hunting)))

(event Custom|Test%20Spawner%20Move
  ;[1 0.241 0.7891] Simple test movement so enemies move from spawner to allow more to spawn
)

(event Custom|Move%20to%20puppy
  (bind _asplayer (Utilities|Casting|CastToPlayer (Game|GetPlayerCharacter 0)))
  (bind _outactors (Actor|GetAllActorsOfClass "/Game/BulePrints/BPC_BaseDog.BPC_BaseDog_C"))
  (if (> (Utilities|Array|Length _outactors) 5)
    (if (not (Utilities|Array|ContainsItem (Variables|/Game/Charactors/Player.Player_C|Getdogs%20hunted _asplayer) (.OutItem (Utilities|Array|Random _outactors))))
      (bind _output_get (Variables|Default|Setdog%20Granny%20is%20hunting (.OutItem (Utilities|Array|Random _outactors)) :!label _label))
      (Utilities|Array|Add (Variables|/Game/Charactors/Player.Player_C|Getdogs%20hunted _asplayer) _output_get)
      (AI|AIMoveTo self "0, 0, 0" _output_get 5.0 false
        (:OnSuccess
          (Development|PrintString "found them")
          (Utilities|FlowControl|Delay 5.0)
          (Utilities|Array|RemoveItem (Variables|/Game/Charactors/Player.Player_C|Getdogs%20hunted _asplayer) (Variables|Default|Getdog%20Granny%20is%20hunting))
          (CallFunction|MovetoPuppy))
        (:OnFail
          (Development|PrintString "Whats a puppy?"))))
    (else
      (goto _label))))

(event Custom|Yoink_That_Puppy
  (params (Dog%20hunted :type BPC%20Base%20Dog%20Object%20Reference))
  (Components|StaticMesh|SetStaticMesh (Variables|Default|GetStaticMesh) (Variables|/Script/Engine.StaticMeshComponent|GetStaticMesh (Variables|/Game/BulePrints/BPC_BaseDog.BPC_BaseDog_C|GetDog Dog%20hunted)))
  (Variables|Default|SetHas%20doggo true)
  (Development|PrintString "Yoink"))

(event EventBeginPlay
  (CallFunction|MovetoPuppy))

(fn ConstructionScript)