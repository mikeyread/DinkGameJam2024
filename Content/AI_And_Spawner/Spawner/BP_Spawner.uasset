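; BP_Spawner is an enemy spawner that spawns queued enemy classes at its own transform.
; AddToQueue appends a class and spawns at once if no BP_Master_Enemy overlaps its Sphere, while a looping timer also attempts a spawn without that check.
; Spawn takes the first queue entry and binds to its OnKilled event; On_Enemy_Killed notifies BP_Gamemode.
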(event Custom|Attempt%20Spawning
  (CallFunction|Spawn))

(event Custom|On_Enemy_Killed
  (bind _asbp_gamemode (Utilities|Casting|CastToBP_Gamemode (Game|GetGameMode)))
  (Default|OnEnemyKilled _asbp_gamemode))

(event EventBeginPlay
  (Utilities|Time|SetTimerbyEvent (delegate Custom|Attempt%20Spawning) 2.0 true)
  (Utilities|Casting|CastToBP_Gamemode (Game|GetGameMode)))

(fn ConstructionScript)

(fn Spawn
  (bind _spawnable_queue (Variables|Default|GetSpawnable_Queue))
  ;[0.1059 0.4706 1] Checking if the Queue is empty or is populated
  (if (Utilities|Array|IsValidIndex (Variables|Default|GetSpawnable_Queue))
    ;[0.1059 0.4706 1] If populated takes the first in the queue and spawns it at the spawner, then removing it from Queue
    (bind _returnvalue (Game|SpawnActorfromClass (Utilities|Array|Get(acopy) _spawnable_queue) (Transformation|GetActorTransform) "Undefined" "MultiplyWithRoot" 0 0))
    (EventDispatchers|BindEventtoOnKilled _returnvalue (EventDispatchers|CreateEvent :!event Custom|On_Enemy_Killed))
    (Utilities|Array|RemoveIndex _spawnable_queue)
    (return true)
    (else
      ;[1 0.1666 0.1765] Fails if Empty
      (return false))))

(fn AddtoQueue
  (params (Enemyclass :type BP%20Master%20Enemy%20Class%20Reference%20%28by%20ref%29))
  (Utilities|Array|Add (Variables|Default|GetSpawnable_Queue) Enemyclass)
  (if (not (Utilities|Array|IsValidIndex (Collision|GetOverlappingActors (Variables|Default|GetSphere) "/Game/AI_And_Spawner/AI/Enemies/BP_Master_Enemy.BP_Master_Enemy_C" :!class /Script/Engine.PrimitiveComponent)))
    (CallFunction|Spawn)))