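; Base dog pawn that picks a random mesh from DogTypes on BeginPlay and wanders the level.
; PuppyRoam uses AI MoveTo to reach random nearby points, pausing and repeating only when a move succeeds.
; Idle loops a timeline that scales the mesh in X and Y, while BeinPet activates a Hearts effect.
; A pitch-wobble chain is left unconnected.
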(event Custom|BeinPet
  (Components|Activation|Activate (Variables|Default|GetHearts) true))

(event Custom|Puppy%20Roam
  (AI|AIMoveTo self (.RandomLocation (AI|Navigation|GetRandomReachablePointinRadius (Transformation|GetActorLocation) 1e+03 0 0)) 0 5.0 false
    (:OnSuccess
      (Utilities|FlowControl|Delay 2.0)
      (CallFunction|PuppyRoam))))

(event Custom|Idle
  (bind (_direction _x_scale _y_scale) (Timeline|Timeline PlayFromStart)
    (:Update
      (Transformation|SetRelativeScale3D (Variables|Default|GetDog) (Math|Vector|MakeVector _x_scale _y_scale 1.0)))
    (:Finished
      (Utilities|FlowControl|Delay 1e-05)
      (Timeline|Timeline PlayFromStart))))

(event EventBeginPlay
  (Utilities|FlowControl|Sequence
    (:then_0
      (Components|StaticMesh|SetStaticMesh (Variables|Default|GetDog) (.OutItem (Utilities|Array|Random (Variables|Default|GetDogTypes)))))
    (:then_1
      (CallFunction|PuppyRoam)
      (CallFunction|Idle))))

(event EventTick
  (params (DeltaSeconds :type Float%20%28single-precision%29))
  (if (and false false)
    _))

(fn ConstructionScript)