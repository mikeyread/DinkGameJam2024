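; Game mode that runs endless enemy waves through the level's BP_Spawner actors.
; Each wave loads a class-to-count enemy pool from DT_Wave_pool_Data by wave number, falling back to random wave-scaled counts.
; Random pool picks are queued on random spawners up to MaxAmountOfEnemies, with kills triggering refills while enough enemies remain.
; When none remain, Transition starts a timer; EndWave is an empty stub.
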(event EventBeginPlay
  (CallFunction|GetAllSpawners)
  (CallFunction|NewWave))

(fn ConstructionScript)

(fn GetAllSpawners
  (bind _outactors (Actor|GetAllActorsOfClass "/Game/AI_And_Spawner/Spawner/BP_Spawner.BP_Spawner_C"))
  (bind _output_get (Variables|Default|SetSpawners _outactors))
  (for _array_element _output_get
    (if (not (Variables|/Game/AI_And_Spawner/Spawner/BP_Spawner.BP_Spawner_C|GetIsOn _array_element))
      (Utilities|Array|RemoveItem (Variables|Default|GetSpawners) _array_element))))

(fn StartWave
  (CallFunction|BuildEnemyPool)
  (for _index (range 0 (- (Math|Integer|Min(Integer) (CallFunction|GetSizeOfEnemyPool) (Variables|Default|GetMax%20Amount%20of%20Enemies)) 1))
    (bind _enemy (CallFunction|GetEnemy))
    (Default|AddtoQueue (.OutItem (Utilities|Array|Random (Variables|Default|GetSpawners))) _enemy)))

(fn NewWave
  (Math|Integer|IncrementInt (Variables|Default|GetWave%20Count)
    (:%20%20
      (CallFunction|GetAllSpawners)
      (CallFunction|StartWave))))

(fn EndWave)

(fn Transition
  (params (TransitionTime :type Float%20%28single-precision%29))
  (bind _returnvalue (Utilities|Time|SetTimerbyEvent (EventDispatchers|CreateEvent :!event NewWave) TransitionTime))
  (Variables|Default|SetTransition_timer _returnvalue))

(fn BuildEnemyPool
  (bind _returnvalue (Utilities|GetDataTableRow "/Game/AI_And_Spawner/Spawner/DT_Wave_pool_Data.DT_Wave_pool_Data" (Utilities|String|StringToName (Utilities|String|ToString(Integer) (Variables|Default|GetWave%20Count))))
    (:then
      (Variables|Default|SetEnemy_Pool (Utilities|Struct|BreakS_Wave _returnvalue))
      (Variables|Default|SetRemaining_Enemies (CallFunction|GetSizeOfEnemyPool)))
    (:RowNotFound
      (Utilities|Map|Add (Variables|Default|GetEnemy_Pool) "/Game/AI_And_Spawner/AI/Enemies/BP_Master_Enemy.BP_Master_Enemy_C" (Math|Random|RandomIntegerinRange 10 (* (Variables|Default|GetWave%20Count) 3)))
      (Utilities|Map|Add (Variables|Default|GetEnemy_Pool) "/Game/AI_And_Spawner/AI/Enemies/BP_Enemy_Child.BP_Enemy_Child_C" (Math|Random|RandomIntegerinRange 5 (* (Variables|Default|GetWave%20Count) 2)))
      (Variables|Default|SetRemaining_Enemies (CallFunction|GetSizeOfEnemyPool)))))

(fn GetSizeOfEnemyPool
  (bind _values (Utilities|Map|Values (Variables|Default|GetEnemy_Pool)))
  (for _array_element _values
    (LocalVariables|SetSum_Local (+ (LocalVariables|GetSum_Local) _array_element)))
  (return (LocalVariables|GetSum_Local)))

(fn GetEnemy
  (bind _enemy_pool (Variables|Default|GetEnemy_Pool))
  (bind _keys (Utilities|Map|Keys (Variables|Default|GetEnemy_Pool)))
  (bind _output_get (LocalVariables|SetLocal_Class_Choice (.OutItem (Utilities|Array|Random _keys))))
  (if (> (- (.Value (Utilities|Map|Find (Variables|Default|GetEnemy_Pool) _output_get)) 1) 0)
    (Utilities|Map|Add _enemy_pool (LocalVariables|GetLocal_Class_Choice) (- (.Value (Utilities|Map|Find (Variables|Default|GetEnemy_Pool) _output_get)) 1))
    (return (LocalVariables|GetLocal_Class_Choice))
    (else
      (Utilities|Map|Remove _enemy_pool (LocalVariables|GetLocal_Class_Choice))
      (return (LocalVariables|GetLocal_Class_Choice)))))

(fn OnEnemyKilled
  (bind _result (Math|Integer|DecrementInt (Variables|Default|GetRemaining_Enemies))
    (:%20%20
      (if (< _result (Variables|Default|GetMax%20Amount%20of%20Enemies))
        (if (<= (Variables|Default|GetRemaining_Enemies) 0)
          (CallFunction|Transition 0.0))
        (else
          (bind _enemy (CallFunction|GetEnemy))
          (Default|AddtoQueue (.OutItem (Utilities|Array|Random (Variables|Default|GetSpawners))) _enemy))))))